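; Player controller for GammaFlow that manages the local player's HUD, menus, indicator sprite and character selection.
; Each tick rotates the indicator toward input and facing, scales it by prefire charge and camera distance, and places it by screen projection (IsOffScreen actually returns true on-screen).
; Character swaps spawn and possess one of three fighters at the camera.
; Lobby, solo and bot starts route to GammaGameInstance; slow-motion rematches to BP_Match.
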(event Custom|SwapCharacter
  (bind _self self)
  (bind _returnvalue (Pawn|GetControlledPawn _self))
  ;[0 0 0] Character Select
  (Utilities|IsValid _returnvalue
    (:Is%20Valid
      (bind _asgamma_character (Utilities|Casting|CastToGammaCharacter _returnvalue))
      (Class|GammaCharacter|ClearFlash _asgamma_character)
      (Utilities|IsValid _asgamma_character
        (:Is%20Valid
          (Development|PrintString (Utilities|GetDisplayName _asgamma_character))
          (bind _output_get (Variables|Default|SetPerviousCharacter _asgamma_character))
          (CallFunction|CharacterSwapInterchange)
          (Actor|DestroyActor _output_get)
          (bind _outactors (Actor|GetAllActorsOfClass "/Game/Blueprints/GammaFlow/BP_Match.BP_Match_C"))
          (Class|GMatch|ClearPlayers (Utilities|Array|Get(acopy) _outactors))
          (Development|PrintString "PAWN IS valid"))))
    (:Is%20Not%20Valid
      (CallFunction|CharacterSwapInterchange)
      (Development|PrintString "pawn not valid"))))

(event Custom|Player_RemoveMenu
  ;[0 0 0] Inter-Network Menu Scrapping
  (if (Variables|Default|GetbRun)
    (Widget|RemovefromParent (Variables|Default|GetPlayer_OnlineMenu))
    (Development|PrintString "REMOVED HUD" true true "(R=0.000000,G=0.100269,B=0.333333,A=1.000000)" 1e+02)
    (else
      (Development|PrintString "REMOVE HUD DROPPED" true true "(R=0.302083,G=0.239038,B=0.000000,A=1.000000)" 1e+02))))

(event Custom|Player_Client_CreateHUD
  ;[0 0 0] HUDs creation function
  (bind _returnvalue (UserInterface|CreateWidget "/Game/Widgets/ChargeBars.ChargeBars_C" self))
  (bind _output_get (Variables|Default|SetGameHud _returnvalue))
  (Utilities|IsValid _output_get
    (:Is%20Valid
      (UserInterface|Viewport|AddtoViewport _output_get 0)
      (Widget|SetVisibility _output_get "Visible")
      (bind _returnvalue_2 (UserInterface|CreateWidget "/Game/Widgets/MainMenu.MainMenu_C" self))
      (bind _output_get_2 (Variables|Default|SetPlayer_OnlineMenu _returnvalue_2))
      (Utilities|IsValid _output_get_2
        (:Is%20Valid
          (UserInterface|Viewport|AddtoViewport _output_get_2 0)
          (Widget|SetVisibility _output_get_2 "Visible")
          (Input|SetInputModeGameandUI (Game|GetPlayerController 0) (Variables|Default|GetPlayer_OnlineMenu) "DoNotLock" true)
          (Variables|Default|SetbShowMouseCursor true))))))

(event Custom|Player_Server_JoinLobby
  ;[0 0.01702 0.07292] Call JoinLobby from our GameInstance BP
  (bind _asgamma_game_instance (Utilities|Casting|CastToGammaGameInstance (Game|GetGameInstance))
    (:then
      (Default|InstanceJoinLobby _asgamma_game_instance self))
    (:CastFailed
      (Development|PrintString "CTRLLR JOIN DROPPED" true true "(R=0.276042,G=0.217570,B=0.000000,A=1.000000)" 1e+02))))

(event Custom|InitializeSolo
  (bind _returnvalue (Game|GetGameInstance))
  ;[0 0 0] SOLO & BOT FIGHT
  (Utilities|IsValid _returnvalue
    (:Is%20Valid
      (bind _asgamma_game_instance (Utilities|Casting|CastToGammaGameInstance _returnvalue))
      (Default|InstanceStartSolo _asgamma_game_instance self (Variables|Default|GetCharacterIndex)))))

(event Custom|EnterNewCharacterIndex
  (params (NewIndex :type Integer))
  ;[0 0 0] Set Character choice 'index' from menu
  (Variables|Default|SetCharacterIndex NewIndex))

(event Custom|CallMenu
  (bind _player_onlinemenu (Variables|Default|GetPlayer_OnlineMenu))
  ;[0 0 0] Player hit "OpenMenu"
  (if (Variables|Default|GetbRun)
    (Utilities|IsValid _player_onlinemenu
      (:Is%20Valid
        (if (Utilities|Enum|Equal(Enum) (Widget|GetVisibility _player_onlinemenu) "Visible")
          (Widget|SetVisibility _player_onlinemenu "Hidden")
          (Input|SetInputModeGameOnly self)
          (Variables|Default|SetbShowMouseCursor false)
          (else
            (Widget|SetVisibility _player_onlinemenu "Visible")
            (Input|SetInputModeGameandUI self (Variables|Default|GetPlayer_OnlineMenu) "DoNotLock" true)
            (Variables|Default|SetbShowMouseCursor true)))))
    (else
      (Development|PrintString "MENU BOOTING" true true "(R=0.000000,G=0.312500,B=0.099404,A=1.000000)" 1e+02))))

(event Custom|CallRoster
  (bind _self self)
  (bind _player_rostermenu (Variables|Default|GetPlayer_RosterMenu))
  ;[0 0 0] Player hit "Show Roster"
  (if (Variables|Default|GetbRun)
    (if (Utilities|Enum|Equal(Enum) (Widget|GetVisibility _player_rostermenu) "Visible")
      (Widget|SetVisibility _player_rostermenu "Hidden")
      (Input|SetInputModeGameOnly _self)
      (Variables|Default|SetbShowMouseCursor false)
      (else
        (Widget|SetVisibility (Variables|Default|GetPlayer_OnlineMenu) "Hidden")
        (Widget|SetVisibility _player_rostermenu "Visible")
        (Input|SetInputModeGameandUI _self (Variables|Default|GetPlayer_RosterMenu) "DoNotLock" true)
        (Variables|Default|SetbShowMouseCursor true)))
    (else
      (Development|PrintString "open roster failed :(" true true "(R=0.000000,G=0.338542,B=0.107688,A=1.000000)" 1e+02))))

(event Custom|CaretUpdate2
  (bind _returnvalue (Game|GetPlayerCharacter 0))
  (bind _returnvalue_2 (Game|GetPlayerCharacter 0))
  (bind _playerindicatorsprite (Variables|Default|GetPlayerIndicatorSprite))
  (bind _returnvalue_3 (Transformation|GetActorLocation _returnvalue))
  ;[0 0 0] CaretUpdate2
  (bind _asgamma_character (Utilities|Casting|CastToGammaCharacter _returnvalue_2))
  (Utilities|IsValid _asgamma_character
    (:Is%20Valid
      (if (> (Math|Vector|VectorLength (Math|Vector|MakeVector (Math|Float|Clamp(Float) (Variables|/Script/Gamma.GammaCharacter|GetInputX _asgamma_character) -1.0) 0.0 (Math|Float|Clamp(Float) (Variables|/Script/Gamma.GammaCharacter|GetInputZ _asgamma_character) -1.0))) 0.0)
        ;;[0 0 0] Rotate to Point to Player
        (Utilities|IsValid _playerindicatorsprite
          (:Is%20Valid
            (Transformation|SetWorldRotation _playerindicatorsprite (Math|Rotator|MakeRotator 0.0 (.Pitch (Math|Rotator|BreakRotator (Math|Rotator|MakeRotfromX (- (+ _returnvalue_3 (Math|Vector|Normalize (Math|Vector|MakeVector (+ (* (Math|Float|Clamp(Float) (Variables|/Script/Gamma.GammaCharacter|GetInputX _asgamma_character) -1.0) 0.5) (.X (Math|Vector|BreakVector (Transformation|GetActorForwardVector _returnvalue_2)))) 1.0 (* (Math|Float|Clamp(Float) (Variables|/Script/Gamma.GammaCharacter|GetInputZ _asgamma_character) -1.0) 0.6)))) _returnvalue_3)))) (.Yaw (Math|Rotator|BreakRotator (Math|Rotator|MakeRotfromX (- (+ _returnvalue_3 (Math|Vector|Normalize (Math|Vector|MakeVector (+ (* (Math|Float|Clamp(Float) (Variables|/Script/Gamma.GammaCharacter|GetInputX _asgamma_character) -1.0) 0.5) (.X (Math|Vector|BreakVector (Transformation|GetActorForwardVector _returnvalue_2)))) 1.0 (* (Math|Float|Clamp(Float) (Variables|/Script/Gamma.GammaCharacter|GetInputZ _asgamma_character) -1.0) 0.6)))) _returnvalue_3))))) false false)))))))

(event Custom|ServerCallRematch
  ;[0 0 0] REMATCH
  (bind _outactors (Actor|GetAllActorsOfClass "/Game/Blueprints/GammaFlow/BP_Match.BP_Match_C"))
  (for _array_element _outactors
    (Utilities|IsValid _array_element
      (:Is%20Valid
        (Default|MatchRematch _array_element)))))

(event Custom|InitializeBotFight
  (bind _returnvalue (Game|GetGameInstance))
  ;[0 0 0] SOLO & BOT FIGHT
  (Utilities|IsValid _returnvalue
    (:Is%20Valid
      (bind _asgamma_game_instance (Utilities|Casting|CastToGammaGameInstance _returnvalue))
      (Default|InstanceStartBotFight _asgamma_game_instance))))

(event Custom|CharacterSwapInterchange
  (bind _playercameramanager (Variables|Default|GetPlayerCameraManager))
  (bind _returnvalue (Camera|GetCameraLocation _playercameramanager))
  (bind (_x _y _z) (Math|Vector|BreakVector _returnvalue))
  (bind _returnvalue_2 (Math|Vector|MakeVector _x 0.0 _z))
  (bind _returnvalue_3 (Math|Transform|MakeTransform _returnvalue_2))
  ;[0 0 0] Character Select
  (switch int (Variables|GammaPlayerController_C|GetCharacterIndex self)
    (:0
      ;[0.1667 0 0] KARAOKE
      (bind _returnvalue_4 (Game|SpawnActorfromClass (Utilities|ResolveSoftReference (Variables|Default|GetKaraoke)) _returnvalue_3 "Undefined" self 0))
      (Utilities|IsValid _returnvalue_4
        (:Is%20Valid
          (Pawn|Possess self _returnvalue_4)
          (Pawn|Input|AddMovementInput _returnvalue_4 "1.000000, 0, 0" 1.0 false)
          (Utilities|IsValid (Variables|/Script/Gamma.GammaCharacter|GetCameraBoom _returnvalue_4)
            (:Is%20Valid
              (Transformation|SetWorldLocation (Variables|/Script/Gamma.GammaCharacter|GetCameraBoom _returnvalue_4) (Transformation|GetActorLocation _returnvalue_4) false false)
              (Input|SetInputModeGameandUI self (Variables|Default|GetPlayer_RosterMenu) "DoNotLock" true)
              (Variables|Default|SetbShowMouseCursor false)
              (CallFunction|AddPlayerIndicator))))))
    (:1
      ;[0 0.1198 0.009734] PEACE GIANT
      (bind _returnvalue_5 (Game|SpawnActorfromClass (Utilities|ResolveSoftReference (Variables|Default|GetPeaceGiant)) _returnvalue_3 "Undefined" self 0))
      (Utilities|IsValid _returnvalue_5
        (:Is%20Valid
          (Pawn|Possess self _returnvalue_5)
          (Pawn|Input|AddMovementInput _returnvalue_5 "1.000000, 0, 0" 1.0 false)
          (Input|SetInputModeGameandUI self (Variables|Default|GetPlayer_RosterMenu) "DoNotLock" true)
          (Variables|Default|SetbShowMouseCursor false)
          (CallFunction|AddPlayerIndicator))))
    (:2
      ;[0.1356 0 0.4948 0.5] BAETYLUS
      (bind _returnvalue_6 (Game|SpawnActorfromClass (Utilities|ResolveSoftReference (Variables|Default|GetBaetylus)) _returnvalue_3 "Undefined" self 0))
      (Utilities|IsValid _returnvalue_6
        (:Is%20Valid
          (Pawn|Possess self _returnvalue_6)
          (Pawn|Input|AddMovementInput _returnvalue_6 "1.000000, 0, 0" 1.0 false)
          (Input|SetInputModeGameandUI self (Variables|Default|GetPlayer_RosterMenu) "DoNotLock" true)
          (Variables|Default|SetbShowMouseCursor false)
          (CallFunction|AddPlayerIndicator))))))

(event Custom|UpdatePlayerIndicator
  (bind _returnvalue (Game|GetPlayerCharacter 0))
  (bind _returnvalue_2 (Game|GetPlayerCameraManager 0))
  (bind _returnvalue_3 (Game|GetPlayerCharacter 0))
  (bind _playerindicatorsprite (Variables|Default|GetPlayerIndicatorSprite))
  (bind _returnvalue_4 (Math|Vector|GetForwardVector _playerindicatorsprite))
  (bind _returnvalue_5 (Transformation|GetActorLocation _returnvalue_3))
  (bind _relativescale3d (Variables|/Script/Engine.SceneComponent|GetRelativeScale3D _playerindicatorsprite))
  (bind _returnvalue_6 (Math|Vector|VectorLength _relativescale3d))
  (bind _returnvalue_7 (+ _returnvalue_5 "0, 0,15.000000"))
  (bind _returnvalue_8 (* _returnvalue_6 15.0))
  (bind _returnvalue_9 (+ _returnvalue_8 1e+02))
  (bind _returnvalue_10 (* _returnvalue_4 _returnvalue_9))
  (bind _returnvalue_11 (+ _returnvalue_7 _returnvalue_10))
  ;[0 0 0] UPDATE PLAYER LOCATOR
  (Utilities|IsValid (Game|GetPlayerCharacter 0)
    (:Is%20Valid
      (Utilities|IsValid (Variables|Default|GetPlayerIndicatorSprite)
        (:Is%20Valid
          ;;[0 0 0] Scaling relative to distance from camera
          (bind _asgamma_character (Utilities|Casting|CastToGammaCharacter _returnvalue))
          (Utilities|IsValid _asgamma_character
            (:Is%20Valid
              (Transformation|SetRelativeScale3D (Variables|Default|GetPlayerIndicatorSprite) (* (Math|Vector|MakeVector (+ (Math|Float|Clamp(Float) (* (Math|Float|Square (Variables|/Script/Gamma.GammaCharacter|GetPrefireTimer _asgamma_character)) 2.0) 0.1) 0.5) 0.15 0.15) (* (Math|Float|Sqrt (Transformation|GetDistanceTo _returnvalue (Game|GetPlayerCameraManager 0))) 0.068)))
              ;;[0 0 0] OFF-SCREEN -- Hug the edge
              (bind _result (CallFunction|GetPlayerScreenPosition))
              (bind _result_2 (CallFunction|IsOffScreen (.X (Math|Vector2D|BreakVector2D _result)) (.Y (Math|Vector2D|BreakVector2D _result))))
              (if _result_2
                ;;[0 0 0] ON-SCREEN -- Positioning relative to player velocity
                (Transformation|SetWorldLocation (Variables|Default|GetPlayerIndicatorSprite) _returnvalue_11 false false)
                (Variables|Default|SetIndicatorPos _returnvalue_11)
                (else
                  (bind _asgamma_character_2 (Utilities|Casting|CastToGammaCharacter (Game|GetPlayerCharacter 0))
                    (:then
                      (Transformation|SetWorldLocation (Variables|Default|GetPlayerIndicatorSprite) (+ (* (- (Transformation|GetActorLocation (Game|GetPlayerCharacter 0)) (+ (Camera|GetCameraLocation _returnvalue_2) (* (Transformation|GetActorForwardVector _returnvalue_2) (Variables|/Script/Engine.SpringArmComponent|GetTargetArmLength (Variables|/Script/Gamma.GammaCharacter|GetCameraBoom _asgamma_character_2))))) 0.25) (+ (Camera|GetCameraLocation _returnvalue_2) (* (Transformation|GetActorForwardVector _returnvalue_2) (Variables|/Script/Engine.SpringArmComponent|GetTargetArmLength (Variables|/Script/Gamma.GammaCharacter|GetCameraBoom _asgamma_character_2))))) false false))
                    (:CastFailed
                      (Development|PrintString "cast failed!" true true "(R=0.000000,G=0.660000,B=1.000000,A=1.000000)" 0.0))))))))))))

(event Custom|AddPlayerIndicator
  (bind _returnvalue (Pawn|GetControlledPawn))
  ;[0 0 0] ADD PLAYER INDICATOR
  (if (not (Actor|ActorHasTag _returnvalue "Spectator"))
    (bind _returnvalue_2 (AddComponent|AddPaperSpriteComponent _returnvalue false (Math|Transform|MakeTransform (Math|Vector|MakeVector 0.0 0.0 -101.0) "0, 0, 0" "0.500000,0.500000,0.500000")))
    (bind _output_get (Variables|Default|SetPlayerIndicatorSprite _returnvalue_2))
    (bind _asgamma_character (Utilities|Casting|CastToGammaCharacter (Game|GetPlayerCharacter 0)))
    (Utilities|IsValid _asgamma_character
      (:Is%20Valid
        (Collision|SetCollisionEnabled _output_get "NoCollision")
        (Variables|/Script/Engine.PrimitiveComponent|SetbGenerateOverlapEvents _output_get false)
        (Variables|/Script/Engine.PrimitiveComponent|SetCanCharacterStepUpOn _output_get "ECB_No")
        (Rendering|Material|SetMaterial _output_get 0 "/Game/Materials/M_PLayerIndicator.M_PlayerIndicator")
        (Variables|Default|SetIndicatorBasePosition (- (Transformation|GetWorldLocation _output_get) (Transformation|GetActorLocation _returnvalue)))))))

(event Custom|Player_Server_HostLobby
  ;[0.09896 0 0] Call HostLobby from our GameInstance BP
  (bind _asgamma_game_instance (Utilities|Casting|CastToGammaGameInstance (Game|GetGameInstance))
    (:then
      (Default|InstanceHostLobby _asgamma_game_instance self))
    (:CastFailed
      (Development|PrintString "CTRLLR HOST DROPPED" true true "(R=0.375000,G=0.295566,B=0.000000,A=1.000000)" 1e+02))))

(event Custom|UpdateTimescale
  (params (DeltaTime :type Float%20%28single-precision%29))
  (if (< (Variables|Default|GetCustomTimeDilation) 1.0)
    (bind _output_get (Variables|Default|SetCustomTimeDilation (Math|Interpolation|FInterpTo (Variables|Default|GetCustomTimeDilation) 1.0 DeltaTime (* (Variables|Default|GetCustomTimeDilation) 15.0))))
    (Development|PrintString (Utilities|String|ToString(Float) _output_get) true true "(R=0.000000,G=1.000000,B=0.447550,A=1.000000)")))

(event EventBeginPlay
  ;[0 0 0] Wait 2 sec, then Create Main Menu and set bRun
  (Utilities|FlowControl|Delay 0.04)
  (Utilities|IsValid (Game|GetPlayerCharacter 0)
    (:Is%20Valid
      (if (Pawn|IsLocalPlayerController)
        (CallFunction|PlayerClientCreateHUD)
        (CallFunction|AddPlayerIndicator)
        (Variables|Default|SetbRun true)
        (else
          (Development|PrintString "Controller not local ;D"))))
    (:Is%20Not%20Valid
      (Development|PrintString "Player Invalid :("))))

(event EventTick
  (params (DeltaSeconds :type Float%20%28single-precision%29))
  ;[0 0 0] TICK
  (CallFunction|UpdatePlayerIndicator)
  (CallFunction|CaretUpdate2))

(event Input|ActionEvents|InputActionOpenMenu
  (params (Key :type Key%20Structure))
  ;[0 0 0] Player hit "OpenMenu"
  (:Pressed
    (CallFunction|CallMenu)))

(event Input|ActionEvents|InputActionOpenRoster
  (params (Key :type Key%20Structure))
  ;[0 0 0] Player hit "Show Roster"
  (:Pressed
    (CallFunction|CallRoster)))

(event Input|ActionEvents|InputActionRematch
  (params (Key :type Key%20Structure))
  ;[0 0 0] REMATCH
  (:Pressed
    (Development|PrintString "SEEN")
    (if (<= (Class|GameplayStatics|GetGlobalTimeDilation) 0.5)
      (CallFunction|ServerCallRematch)
      (Development|PrintString "RESTARTING..."))))

(fn ConstructionScript)

(fn IsOffScreen
  (params (x :type Float%20%28single-precision%29) (y :type Float%20%28single-precision%29))
  (bind _returnvalue (Game|GetPlayerController 0))
  (bind (_sizex _sizey) (HUD|GetViewportSize _returnvalue))
  (return (and (and (> x 0.0) (> y 0.0)) (and (< x (Math|Conversions|ToFloat(Integer) _sizex)) (< y (Math|Conversions|ToFloat(Integer) _sizey))))))

(fn GetPlayerScreenPosition
  (return (.ScreenPosition (Class|GameplayStatics|ProjectWorldtoScreen (Game|GetPlayerController 0) (Transformation|GetWorldLocation (Variables|/Script/Engine.Actor|GetRootComponent (Game|GetPlayerCharacter 0))) false))))