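; Match manager for GammaFlow that handles the "GAME!" ending, slow-motion effects and rematches.
; On authority, Tick waits for GG and slowed global time, then spawns the plate at the local player and applies GG timescale; UpdateHitConfirm slows both players on MinorGG.
; MatchRematch clears combat actors and the plate, resets and scatters characters around the camera, and restores time.
; Spectator-tagged levels auto-restart after a dilation-scaled delay.
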(event Custom|ClearDoomedActors
  ;[0 0 0] Clear Doomed Actors
  (bind _outactors (Actor|GetAllActorswithTag "Doomed"))
  (if (> (Utilities|Array|Length _outactors) 0)
    (for _array_element _outactors
      (Utilities|IsValid _array_element
        (:Is%20Valid
          (bind _asgamma_character (Utilities|Casting|CastToGammaCharacter _array_element)
            (:then
              (Class|GammaCharacter|NullifyAttack _asgamma_character)
              (Class|GammaCharacter|NullifySecondary _asgamma_character)
              (Actor|DestroyActor _asgamma_character))
            (:CastFailed
              (Actor|DestroyActor _array_element))))))))

(event Custom|CreateGGPlate
  ;[0 0 0] Create gg plate
  (bind _returnvalue (Class|GMatch|GetLocalPlayer))
  (Utilities|IsValid _returnvalue
    (:Is%20Valid
      (bind _returnvalue_2 (Game|SpawnActorfromClass "/Game/Blueprints/GammaFlow/BP_GAME_Plate.BP_GAME_Plate_C" (Math|Transform|MakeTransform (Math|Vector|MakeVector (.X (Math|Vector|BreakVector (Transformation|GetActorLocation _returnvalue))) -5e+01 (.Z (Math|Vector|BreakVector (Transformation|GetActorLocation _returnvalue))))) "Undefined" 0 0))
      (CallFunction|Timescale)
      (Utilities|IsValid _returnvalue_2
        (:Is%20Valid
          ;[0 0 0] AUTO-RESTART for Watch Mode
          (if (Variables|Default|GetbSpectatorGame)
            (Development|PrintString "AUTO-RESTARTING..." true true "(R=0.000000,G=0.660000,B=1.000000,A=1.000000)" 0.025)
            (Utilities|FlowControl|Delay (* 3.0 (Class|GameplayStatics|GetGlobalTimeDilation)))
            (Development|PrintString "..DONE" true true "(R=0.000000,G=0.660000,B=1.000000,A=1.000000)" 0.025)
            (CallFunction|MatchRematch)))))
    (:Is%20Not%20Valid
      (Development|PrintString "LOCAL PLAYER NON VALID"))))

(event Custom|UpdateHitConfirm
  (Networking|SwitchHasAuthority
    (:Authority
      (if (Variables|Default|GetbMinorGG)
        (Development|PrintString "match setting timescale")
        (CallFunction|SetTimescales)
        (Variables|Default|SetbMinorGG false)))))

(event Custom|Clear%20Flashes
  (bind _outactors (Actor|GetAllActorsOfClass "/Script/Gamma.GFlash"))
  (if (> (Utilities|Array|Length _outactors) 0)
    (for _array_element _outactors
      (Utilities|IsValid _array_element
        (:Is%20Valid
          (Actor|DestroyActor _array_element))))))

(event Custom|Timescale
  ;[0 0 0] Set Timescale to GG time
  (Utilities|Time|SetGlobalTimeDilation (Variables|Default|GetGGTimescale)))

(event Custom|MatchRematch
  ;[0 0 0] RESTART - Reset time, replace players, clear gg plate
  (CallFunction|ResetPlayers)
  (CallFunction|ClearAttacks)
  (CallFunction|ClearFlashes)
  (CallFunction|ClearDoomedActors)
  (CallFunction|ClearGGPlate)
  (Variables|Default|SetbGGInProgress false)
  (Variables|Default|SetbGG false)
  (Utilities|Time|SetGlobalTimeDilation (Variables|Default|GetNaturalTimeScale))
  (Networking|ForceNetUpdate))

(event Custom|SetTimescales
  (bind _returnvalue (Class|GMatch|GetLocalPlayer))
  (Utilities|IsValid _returnvalue
    (:Is%20Valid
      (bind _returnvalue_2 (Class|GMatch|GetOpponentPlayer))
      (Utilities|IsValid _returnvalue_2
        (:Is%20Valid
          (Variables|/Script/Engine.Actor|SetCustomTimeDilation _returnvalue 0.1)
          (Variables|/Script/Engine.Actor|SetCustomTimeDilation _returnvalue_2 0.1)
          (Variables|Default|SetbMinorGG false))))))

(event Custom|ResetPlayers
  (bind _returnvalue (Game|GetPlayerCameraManager 0))
  (bind _returnvalue_2 (Camera|GetCameraLocation _returnvalue))
  (bind (_x _y _z) (Math|Vector|BreakVector _returnvalue_2))
  (bind _outactors (Actor|GetAllActorsOfClass "/Script/Gamma.GammaCharacter"))
  (if (> (Utilities|Array|Length _outactors) 0)
    (for (_array_element _array_index) _outactors
      (Utilities|IsValid _array_element
        (:Is%20Valid
          (bind _asgamma_character (Utilities|Casting|CastToGammaCharacter _array_element))
          (Variables|/Script/Engine.Actor|SetCustomTimeDilation _asgamma_character 1.1)
          (Class|GammaCharacter|EraseCharge _asgamma_character)
          (Class|GammaCharacter|ResetLocator _asgamma_character)
          (Transformation|SetActorLocation _array_element (+ (Math|Vector|MakeVector (* _array_index (Math|Random|RandomFloatinRange 2e+02 2e+03)) 0.0 (* _array_index (Math|Random|RandomFloatinRange 5.0 5e+02))) (Math|Vector|MakeVector _x 0.0 _z)) false false)
          (Pawn|Input|AddMovementInput _asgamma_character "1.000000, 0, 0" 1.0 false)
          (Class|GammaCharacter|ModifyHealth _asgamma_character 1e+03)
          (Class|GammaCharacter|ResetFlipbook _asgamma_character)
          (Class|GammaCharacter|NullifyAttack _asgamma_character)
          (Class|GammaCharacter|NullifySecondary _asgamma_character))))))

(event Custom|Clear%20GG%20Plate
  ;[0 0 0] Clear GG Plate
  (bind _outactors (Actor|GetAllActorsOfClass "/Game/Blueprints/GammaFlow/BP_GAME_Plate.BP_GAME_Plate_C"))
  (if (> (Utilities|Array|Length _outactors) 0)
    (Utilities|IsValid (Utilities|Array|Get(acopy) _outactors)
      (:Is%20Valid
        (Actor|DestroyActor (Utilities|Array|Get(acopy) _outactors))))))

(event Custom|Clear%20Attacks
  (bind _outactors (Actor|GetAllActorsOfClass "/Script/Gamma.GAttack"))
  (if (> (Utilities|Array|Length _outactors) 0)
    (for _array_element _outactors
      (Utilities|IsValid _array_element
        (:Is%20Valid
          (Class|GAttack|Nullify _array_element -1))))))

(event EventBeginPlay
  (bind _outactors (Actor|GetAllActorswithTag "Spectator"))
  (if (> (Utilities|Array|Length _outactors) 0)
    (Variables|Default|SetbSpectatorGame true)))

(event Collision|EventActorBeginOverlap
  (params (OtherActor :type Actor%20Object%20Reference)))

(event EventTick
  (params (DeltaSeconds :type Float%20%28single-precision%29))
  (Networking|SwitchHasAuthority
    (:Authority
      ;[0 0 0] Catch moment of gg to spawn "GAME!" plate
      (if (Math|Boolean|ANDBoolean (Variables|Default|GetbGG) (not (Variables|Default|GetbGGInProgress)) (<= (Class|GameplayStatics|GetGlobalTimeDilation) (Variables|Default|GetGGTimescale)))
        (CallFunction|CreateGGPlate)
        (Variables|Default|SetbGGInProgress true)))))

(fn ConstructionScript)