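; Game instance that handles mode switching and online sessions for GammaFlow: bot fight, solo, and lobby hosting, searching and joining.
; Bot fight destroys the session before travel; solo uses a delayed hack to close the menu and swap character.
; Hosting creates a non-LAN session and opens a listen-server level.
; Searches cache results in Games; joining attempts every cached session, or searches again when none exist.
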(event Custom|Instance_HostLobby
  (params (Host :type Player%20Controller%20Object%20Reference))
  ;[0 0 0] Create and Host a Lobby
  (bind _returnvalue (Game|GetCurrentLevelName true))
  (|Session Host 5 false
    (:OnSuccess
      (Development|PrintString "CREATE SESSION SUCCESS" true true "(R=0.000000,G=0.241722,B=0.322917,A=1.000000)")
      (Development|PrintString (Utilities|String|Append "OPENING  " (Utilities|String|ToString(Name) (Variables|Default|GetInstance_LevelName))) true true "(R=0.000000,G=0.237187,B=0.359375,A=1.000000)")
      (Game|OpenLevel(byName) (Variables|Default|GetInstance_LevelName) false "listen")
      (Variables|Default|SetbAutoSearch false))
    (:OnFailure
      (Development|PrintString "CREATE SESSION DROPPED" true true "(R=0.333333,G=0.262726,B=0.000000,A=1.000000)"))))

(event Custom|Instance_StartSolo
  (params (Player :type Player%20Controller%20Object%20Reference) (CharacterIndex :type Integer))
  (bind _returnvalue (Game|GetPlayerController 0))
  ;[0 0 0] Solo Mode
  (Variables|Default|SetControllerCharacterIndex CharacterIndex)
  (Game|OpenLevel(byName) (Variables|Default|GetSolo_LevelName) false)
  (Variables|Default|SetbAutoSearch false)
  ;[0 0 0] Super Hacky menu disable for the solo experience
  (Utilities|FlowControl|Delay 0.05)
  (bind _asgamma_player_controller (Utilities|Casting|CastToGammaPlayerController (Game|GetPlayerController 0)))
  (Default|CallMenu _asgamma_player_controller)
  ;[0.09896 0 0] Swap Character
  (bind _asgamma_player_controller_2 (Utilities|Casting|CastToGammaPlayerController (Game|GetPlayerController 0)))
  (Variables|/Game/Blueprints/GammaFlow/GammaPlayerController.GammaPlayerController_C|SetCharacterIndex _asgamma_player_controller_2 (Variables|Default|GetControllerCharacterIndex))
  (Default|SwapCharacter _asgamma_player_controller_2)
  (Input|SetInputModeGameOnly _returnvalue)
  (Variables|/Script/Engine.PlayerController|SetbShowMouseCursor _returnvalue false))

(event Custom|Instance_StartBotFight
  (params (Player :type Player%20Controller%20Object%20Reference))
  ;[0 0 0] Start Bot Fight
  (|DestroySession (Variables|Default|GetController)
    (:then
      (Game|OpenLevel(byName) (Variables|Default|GetBotFight_LevelName))
      (Pawn|UnPossess (Game|GetPlayerController 0)))))

(event Custom|Instance_JoinLobby
  (params (Joining :type Player%20Controller%20Object%20Reference))
  (bind _games (Variables|Default|GetGames))
  ;[0 0 0] Join Lobby
  (if (> (Utilities|Array|Length _games) 0)
    (for _array_element _games
      (Development|PrintString (Class|FindSessionsCallbackProxy|GetServerName _array_element) true true "(R=0.000000,G=0.206250,B=0.312500,A=1.000000)")
      (|JoinSession Joining _array_element
        (:OnSuccess
          (bind _returnvalue (Game|GetCurrentLevelName true))
          (Development|PrintString (Utilities|String|Append "JOINING  " _returnvalue) true true "(R=0.000000,G=0.277545,B=0.375000,A=1.000000)"))
        (:OnFailure
          (Development|PrintString "JOIN SESSION DROPPED" true true "(R=0.352106,G=0.369792,B=0.000000,A=1.000000)"))))
    (else
      (Development|PrintString "NO GAMES FOUND, SEARCHING...")
      (CallFunction|InstanceFindLobbies))))

(event Custom|Instance_FindLobbies
  (params (Joining :type Player%20Controller%20Object%20Reference))
  ;[0 0 0] Find Lobbies
  (Variables|Default|SetbSearching true)
  (bind _results (|FindSessions Joining 15000 false)
    (:then
      (Development|PrintString "FINDING SESSIONS..." true true "(R=0.000000,G=0.230312,B=0.348958,A=1.000000)" 5.0))
    (:OnSuccess
      (if (> (Utilities|Array|Length _results) 0)
        (Variables|Default|SetGames _results)
        (Variables|Default|SetbSearching false)
        (else
          (Development|PrintString "NO SESSIONS FOUND" true true "(R=0.192708,G=0.192708,B=0.192708,A=1.000000)")
          (Variables|Default|SetbSearching false))))
    (:OnFailure
      (Development|PrintString "FIND SESSION DROPPED" true true "(R=0.437500,G=0.355279,B=0.000000,A=1.000000)"))))

(fn GetNumGames
  (return (Utilities|Array|Length (Variables|Default|GetGames))))