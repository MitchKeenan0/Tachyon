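; BP_SwarmCentre is a spawner actor that produces BP_SwarmAttack actors.
; On BeginPlay it spawns an initial batch at random offsets around itself, flattened onto the Y=0 plane.
; Tick then accumulates delta time and spawns another at the centre's own transform whenever the timer reaches SpawnRate, so the swarm keeps growing.
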(event EventBeginPlay
  (bind _returnvalue (Math|Random|RandomUnitVector))
  (bind _returnvalue_2 (Transformation|GetActorTransform))
  (bind (_location _rotation _scale) (Math|Transform|BreakTransform _returnvalue_2))
  (bind _returnvalue_3 (* _returnvalue 1e+03))
  (bind _returnvalue_4 (+ _returnvalue_3 _location))
  (bind (_x _y _z) (Math|Vector|BreakVector _returnvalue_4))
  (for _index (range 0 5)
    (Game|SpawnActorfromClass "/Game/Blueprints/BP_SwarmAttack.BP_SwarmAttack_C" (Math|Transform|MakeTransform (Math|Vector|MakeVector _x 0.0 _z) "0, 0, 0" _scale) "Undefined" 0 0)))

(event Collision|EventActorBeginOverlap
  (params (OtherActor :type Actor%20Object%20Reference)))

(event EventTick
  (params (DeltaSeconds :type Float%20%28single-precision%29))
  (bind _output_get (Variables|Default|SetSpawnTimer (+ DeltaSeconds (Variables|Default|GetSpawnTimer))))
  (if (>= _output_get (Variables|Default|GetSpawnRate))
    (Game|SpawnActorfromClass "/Game/Blueprints/BP_SwarmAttack.BP_SwarmAttack_C" (Transformation|GetActorTransform) "Undefined" 0 0)
    (Variables|Default|SetSpawnTimer 0.0)))

(fn ConstructionScript)