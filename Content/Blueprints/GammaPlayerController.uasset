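; Player controller for Gamma that manages the local player's HUD and menus, lobby requests, character selection and rematches.
; Shortly after BeginPlay it creates charge bars and the online menu, setting Run, which gates menu and roster toggles that switch input mode and cursor.
; Host and join requests forward to GammaGameInstance.
; Character swaps destroy the pawn, clear BP_Match players and possess Karaoke or PeaceGiant by index; rematch also calls BP_Match.
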(event Custom|SwapCharacter
  (bind _self self)
  (bind _self_2 self)
  (bind _returnvalue (Pawn|GetControlledPawn _self))
  ;[0 0 0] Character Select
  (Utilities|IsValid _returnvalue
    (:Is%20Valid
      (bind _asgamma_character (Utilities|Casting|CastToGammaCharacter _returnvalue))
      (Class|GammaCharacter|ClearFlash _asgamma_character)
      (Actor|DestroyActor _returnvalue)
      (bind _outactors (Actor|GetAllActorsOfClass "/Game/Blueprints/BP_Match.BP_Match_C"))
      (Class|GMatch|ClearPlayers (Utilities|Array|Get(acopy) _outactors))
      (switch int (Variables|GammaPlayerController_C|GetCharacterIndex self)
        (:0
          ;[0.1667 0 0] KARAOKE
          (bind _returnvalue_2 (Game|SpawnActorfromClass (Utilities|ResolveSoftReference (Variables|Default|GetKaraoke)) (Math|Transform|MakeTransform "0, 0, 0") "Undefined" 0 0))
          (Pawn|Possess self _returnvalue_2)
          (Input|SetInputModeGameandUI _self_2 (Variables|Default|GetPlayer_RosterMenu) "DoNotLock" true)
          (Variables|Default|SetbShowMouseCursor false))
        (:1
          ;[0 0.1198 0.009734] PEACE GIANT
          (bind _returnvalue_3 (Game|SpawnActorfromClass (Utilities|ResolveSoftReference (Variables|Default|GetPeaceGiant)) (Math|Transform|MakeTransform "0, 0, 0") "Undefined" 0 0))
          (Pawn|Possess self _returnvalue_3)
          (Input|SetInputModeGameandUI _self_2 (Variables|Default|GetPlayer_RosterMenu) "DoNotLock" true)
          (Variables|Default|SetbShowMouseCursor false))))))

(event Custom|Player_RemoveMenu
  ;[0 0 0] Inter-Network Menu Scrapping
  (if (Variables|Default|GetbRun)
    (Widget|RemovefromParent (Variables|Default|GetPlayer_OnlineMenu))
    (Development|PrintString "REMOVED HUD" true true "(R=0.000000,G=0.100269,B=0.333333,A=1.000000)" 1e+02)
    (else
      (Development|PrintString "REMOVE HUD DROPPED" true true "(R=0.302083,G=0.239038,B=0.000000,A=1.000000)" 1e+02))))

(event Custom|Player_Client_CreateHUD
  ;[0 0 0] HUDs creation function
  (bind _returnvalue (UserInterface|CreateWidget "/Game/Widgets/ChargeBars.ChargeBars_C" self))
  (bind _output_get (Variables|Default|SetGameHud _returnvalue))
  (UserInterface|Viewport|AddtoViewport _output_get 0)
  (Widget|SetVisibility _output_get "Visible")
  (bind _returnvalue_2 (UserInterface|CreateWidget "/Game/Widgets/MainMenu.MainMenu_C" self))
  (bind _output_get_2 (Variables|Default|SetPlayer_OnlineMenu _returnvalue_2))
  (UserInterface|Viewport|AddtoViewport _output_get_2 0)
  (Widget|SetVisibility _output_get_2 "Visible")
  (Input|SetInputModeGameandUI (Game|GetPlayerController 0) (Variables|Default|GetPlayer_OnlineMenu) "DoNotLock" true)
  (Variables|Default|SetbShowMouseCursor true))

(event Custom|Player_Server_JoinLobby
  ;[0 0.01702 0.07292] Call JoinLobby from our GameInstance BP
  (bind _asgamma_game_instance (Utilities|Casting|CastToGammaGameInstance (Game|GetGameInstance))
    (:then
      (Default|InstanceJoinLobby _asgamma_game_instance self))
    (:CastFailed
      (Development|PrintString "CTRLLR JOIN DROPPED" true true "(R=0.276042,G=0.217570,B=0.000000,A=1.000000)" 1e+02))))

(event Custom|InitializeSolo)

(event Custom|EnterNewCharacterIndex
  (params (NewIndex :type Integer))
  ;[0 0 0] Set Character choice 'index' from menu
  (Variables|Default|SetCharacterIndex NewIndex))

(event Custom|CallMenu
  (bind _self self)
  (bind _player_onlinemenu (Variables|Default|GetPlayer_OnlineMenu))
  ;[0 0 0] Player hit "OpenMenu"
  (if (Variables|Default|GetbRun)
    (if (Utilities|Enum|Equal(Enum) (Widget|GetVisibility _player_onlinemenu) "Visible")
      (Widget|SetVisibility _player_onlinemenu "Hidden")
      (Input|SetInputModeGameOnly _self)
      (Variables|Default|SetbShowMouseCursor false)
      (else
        (Widget|SetVisibility _player_onlinemenu "Visible")
        (Input|SetInputModeGameandUI _self (Variables|Default|GetPlayer_OnlineMenu) "DoNotLock" true)
        (Variables|Default|SetbShowMouseCursor true)))
    (else
      (Development|PrintString "MENU BOOTING" true true "(R=0.000000,G=0.312500,B=0.099404,A=1.000000)" 1e+02))))

(event Custom|CallRoster
  (bind _self self)
  (bind _player_rostermenu (Variables|Default|GetPlayer_RosterMenu))
  ;[0 0 0] Player hit "Show Roster"
  (if (Variables|Default|GetbRun)
    (if (Utilities|Enum|Equal(Enum) (Widget|GetVisibility _player_rostermenu) "Visible")
      (Widget|SetVisibility _player_rostermenu "Hidden")
      (Input|SetInputModeGameOnly _self)
      (Variables|Default|SetbShowMouseCursor false)
      (else
        (Widget|SetVisibility (Variables|Default|GetPlayer_OnlineMenu) "Hidden")
        (Widget|SetVisibility _player_rostermenu "Visible")
        (Input|SetInputModeGameandUI _self (Variables|Default|GetPlayer_RosterMenu) "DoNotLock" true)
        (Variables|Default|SetbShowMouseCursor true)))
    (else
      (Development|PrintString "open roster failed :(" true true "(R=0.000000,G=0.338542,B=0.107688,A=1.000000)" 1e+02))))

(event Custom|ServerCallRematch
  ;[0 0 0] REMATCH
  (bind _outactors (Actor|GetAllActorsOfClass "/Game/Blueprints/BP_Match.BP_Match_C"))
  (Default|MatchRematch (Utilities|Array|Get(acopy) _outactors)))

(event Custom|Player_Server_HostLobby
  ;[0.09896 0 0] Call HostLobby from our GameInstance BP
  (bind _asgamma_game_instance (Utilities|Casting|CastToGammaGameInstance (Game|GetGameInstance))
    (:then
      (Default|InstanceHostLobby _asgamma_game_instance self))
    (:CastFailed
      (Development|PrintString "CTRLLR HOST DROPPED" true true "(R=0.375000,G=0.295566,B=0.000000,A=1.000000)" 1e+02))))

(event EventBeginPlay
  ;[0 0 0] Wait 2 sec, then Create Main Menu and set bRun
  (Utilities|FlowControl|Delay 0.1)
  (if (Pawn|IsLocalPlayerController)
    (CallFunction|PlayerClientCreateHUD)
    (Variables|Default|SetbRun true)
    (Development|PrintString "GENERATING HUD" true true "(R=0.000000,G=0.155674,B=0.380208,A=1.000000)")))

(event EventTick
  (params (DeltaSeconds :type Float%20%28single-precision%29)))

(event Input|ActionEvents|InputActionOpenMenu
  (params (Key :type Key%20Structure))
  ;[0 0 0] Player hit "OpenMenu"
  (:Pressed
    (CallFunction|CallMenu)))

(event Input|ActionEvents|InputActionOpenRoster
  (params (Key :type Key%20Structure))
  ;[0 0 0] Player hit "Show Roster"
  (:Pressed
    (CallFunction|CallRoster)))

(event Input|ActionEvents|InputActionRematch
  (params (Key :type Key%20Structure))
  ;[0 0 0] REMATCH
  (:Pressed
    (CallFunction|ServerCallRematch)))

(fn ConstructionScript)