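; Game instance Blueprint that handles multiplayer lobby hosting and joining through online sessions, with on-screen debug prints at each stage.
; Hosting creates a non-LAN session, then reopens the current level as a listen server on success.
; Joining searches for non-LAN sessions and attempts to join every result in a loop rather than selecting one, printing server names and the game count.
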(event Custom|Instance_HostLobby
  (params (Host :type Player%20Controller%20Object%20Reference))
  ;[0 0 0] Create and Host a Lobby
  (bind _returnvalue (Game|GetCurrentLevelName true))
  (bind _output_get (Variables|Default|SetInstance_LevelName (Utilities|String|StringToName _returnvalue)))
  (Development|PrintString (Utilities|String|Append "Level Name  " (Utilities|String|ToString(Name) _output_get)) true true "(R=0.000000,G=0.247500,B=0.375000,A=1.000000)" 1e+02)
  (|Session Host 5 false
    (:OnSuccess
      (Development|PrintString "CREATE SESSION SUCCESS" true true "(R=0.000000,G=0.241722,B=0.322917,A=1.000000)" 1e+02)
      (Development|PrintString (Utilities|String|Append "OPENING  " (Utilities|String|ToString(Name) (Variables|Default|GetInstance_LevelName))) true true "(R=0.000000,G=0.237187,B=0.359375,A=1.000000)" 1e+02)
      (Game|OpenLevel(byName) (Variables|Default|GetInstance_LevelName) true "listen"))
    (:OnFailure
      (Development|PrintString "CREATE SESSION DROPPED" true true "(R=0.333333,G=0.262726,B=0.000000,A=1.000000)" 1e+02))))

(event Custom|Instance_JoinLobby
  (params (Joining :type Player%20Controller%20Object%20Reference))
  ;[0 0 0] Seek and Join a Lobby
  (bind _results (|FindSessions Joining 1500 false)
    (:then
      (Development|PrintString "FINDING SESSIONS..." true true "(R=0.000000,G=0.230312,B=0.348958,A=1.000000)" 1e+02))
    (:OnSuccess
      (if (> (Utilities|Array|Length _results) 0)
        (for _array_element _results
          (Development|PrintString (Class|FindSessionsCallbackProxy|GetServerName _array_element) true true "(R=0.000000,G=0.206250,B=0.312500,A=1.000000)" 1e+02)
          (|JoinSession Joining _array_element
            (:then
              (bind _returnvalue (Game|GetCurrentLevelName true)))
            (:OnSuccess
              (Development|PrintString (Utilities|String|Append "JOIN SUCCESS  " _returnvalue) true true "(R=0.000000,G=0.277545,B=0.375000,A=1.000000)" 1e+02))
            (:OnFailure
              (Development|PrintString "JOIN SESSION DROPPED" true true "(R=0.352106,G=0.369792,B=0.000000,A=1.000000)" 1e+02))))
        (Development|PrintString (Utilities|String|Append "NUM GAMES: " (Utilities|String|ToString(Integer) (Utilities|Array|Length _results))) true true "(R=0.000000,G=0.151250,B=0.229167,A=1.000000)" 1e+02)
        (else
          (Development|PrintString "NO SESSIONS FOUND" true true "(R=0.192708,G=0.192708,B=0.192708,A=1.000000)" 1e+02))))
    (:OnFailure
      (Development|PrintString "FIND SESSION DROPPED" true true "(R=0.437500,G=0.355279,B=0.000000,A=1.000000)" 1e+02))))