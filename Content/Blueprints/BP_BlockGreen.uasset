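; BP_BlockGreen is a short-lived block effect actor with damage particles, sound and a radial force.
; On BeginPlay it plays a strong world camera shake at its location and randomizes the damage sound's pitch.
; During the first half of its lifetime, Tick decays the particles' time dilation each frame, slowing them toward a freeze.
; At the halfway point it negates the radial force strength once, reversing the push or pull.
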(event EventBeginPlay
  ;[0 0 0] Camera Shake
  (Camera|PlayWorldCameraShake "/Game/Blueprints/GammaFlow/BP_StrongCameraShake.BP_StrongCameraShake_C" (Transformation|GetActorLocation) 0.0 2e+03)
  ;[0 0 0] Range-Random Pitch
  (Audio|Components|Audio|SetPitchMultiplier (Variables|Default|GetDamageSound) (Math|Random|RandomFloatinRange 0.15 1.0)))

(event Collision|EventActorBeginOverlap
  (params (OtherActor :type Actor%20Object%20Reference)))

(event EventTick
  (params (DeltaSeconds :type Float%20%28single-precision%29))
  (bind _damageparticles (Variables|Default|GetDamageParticles))
  (bind _radialforce (Variables|Default|GetRadialForce))
  ;[0 0 0] TICK
  (if (> (/ (Variables|Default|GetLifetime) 2.0) (Actor|GetGameTimeSinceCreation))
    (Variables|/Script/Engine.ParticleSystemComponent|SetCustomTimeDilation _damageparticles (* (Variables|/Script/Engine.ParticleSystemComponent|GetCustomTimeDilation _damageparticles) 0.9))
    (elif (not (Variables|Default|GetbVelFlipped))
      (Variables|/Script/Engine.RadialForceComponent|SetForceStrength _radialforce (* (Variables|/Script/Engine.RadialForceComponent|GetForceStrength _radialforce) -1.0))
      (Variables|Default|SetbVelFlipped true))))

(fn ConstructionScript)