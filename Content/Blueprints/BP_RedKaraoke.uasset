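; BP_RedKaraoke is an effect actor that adds two particle systems and animates the scale of its Locator component.
; The Locator starts enlarged on BeginPlay and shrinks geometrically each Tick, independent of delta time, until it is nearly zero.
; Whenever global time dilation drops below the slow-motion threshold, it snaps back to full size and holds there until time speeds up again.
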(event Custom|ResetLocator
  (Transformation|SetRelativeScale3D (Variables|Default|GetLocator) "20.000000,20.000000,20.000000"))

(event Custom|LocatorScaling
  (if (>= (Class|GameplayStatics|GetGlobalTimeDilation) 0.7)
    (if (>= (Math|Vector|VectorLength (Variables|/Script/Engine.SceneComponent|GetRelativeScale3D (Variables|Default|GetLocator))) 0.1)
      (Transformation|SetRelativeScale3D (Variables|Default|GetLocator) (* (Variables|/Script/Engine.SceneComponent|GetRelativeScale3D (Variables|Default|GetLocator)) 0.9)))
    (else
      (CallFunction|ResetLocator))))

(event EventBeginPlay
  (AddComponent|AddParticleSystemComponent false)
  (AddComponent|AddParticleSystemComponent false)
  (CallFunction|ResetLocator))

(event EventTick
  (params (DeltaSeconds :type Float%20%28single-precision%29))
  (CallFunction|LocatorScaling))

(fn ConstructionScript)