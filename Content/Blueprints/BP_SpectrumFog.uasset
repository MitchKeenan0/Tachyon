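; BP_SpectrumFog shifts the default light color of atmospheric fog through a spectrum of colors over time.
; Each Tick derives an index from time since creation scaled by ColourIndez, wrapping over six ColourArray entries.
; The fog color eases toward that entry's OutVal with CInterpTo, whose speed is itself scaled by DeltaSeconds, making blending frame-rate dependent.
; A debug print of the index is left disconnected.
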(event EventBeginPlay)

(event Collision|EventActorBeginOverlap
  (params (OtherActor :type Actor%20Object%20Reference)))

(event EventTick
  (params (DeltaSeconds :type Float%20%28single-precision%29))
  (bind _atmosphericfog (Variables|Default|GetAtmosphericFog))
  (Class|AtmosphericFogComponent|SetDefaultLightColor _atmosphericfog (Class|KismetMathLibrary|CInterpto (Math|Conversions|ToLinearColor(Color) (Variables|/Script/Engine.AtmosphericFogComponent|GetDefaultLightColor _atmosphericfog)) (.OutVal (Utilities|Struct|BreakInterpCurvePointLinearColor (Utilities|Array|Get(acopy) (Variables|Default|GetColourArray) (Math|Integer|%(Integer) (Math|Float|Floor (* (Variables|Default|GetColourIndez) (* (Actor|GetGameTimeSinceCreation) 0.2))) 6)))) DeltaSeconds (* DeltaSeconds 1e+01))))

(fn ConstructionScript)