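; BP_SpearAttack is a spear attack projectile that shakes nearby cameras when it spawns.
; BeginPlay launches it forward at a speed scaled quadratically by AttackMagnitude and ProjectileSpeed.
; Each tick interpolates velocity toward forward max speed, more slowly for larger magnitudes, calls Nullify if it would drop below a threshold, and forces a net update.
; An unconnected branch would spawn child spears for lethal attacks but never runs.
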(event Custom|Accelerate
  (params (DeltaT :type Float%20%28single-precision%29))
  (bind _projectilecomponent (Variables|Default|GetProjectileComponent))
  ;[0 0 0] ACCELERATION
  (if (>= (Math|Vector|VectorLength (Math|Interpolation|VInterptoConstant (Variables|/Script/Engine.MovementComponent|GetVelocity _projectilecomponent) (Variables|Default|GetTargetVector) DeltaT (/ 1e+03 (Variables|Default|GetAttackMagnitude)))) 333.0)
    (Variables|/Script/Engine.MovementComponent|SetVelocity _projectilecomponent (Math|Interpolation|VInterptoConstant (Variables|/Script/Engine.MovementComponent|GetVelocity _projectilecomponent) (Variables|Default|GetTargetVector) DeltaT (/ 1e+03 (Variables|Default|GetAttackMagnitude))))
    (else
      (Class|GAttack|Nullify))))

(event EventBeginPlay
  (bind _projectilespeed (Variables|Default|GetProjectileSpeed))
  (Camera|PlayWorldCameraShake "/Game/Blueprints/GammaFlow/BP_LightCameraShake.BP_LightCameraShake_C" (Transformation|GetActorLocation) 0.0 5555.0)
  (Variables|Default|SetTargetVector (* (Transformation|GetActorForwardVector) (Variables|Default|GetProjectileMaxSpeed)))
  (Variables|/Script/Engine.MovementComponent|SetVelocity (Variables|Default|GetProjectileComponent) (* (Transformation|GetActorForwardVector) (* _projectilespeed (* (* (+ (Variables|Default|GetAttackMagnitude) 1.1) (+ (Variables|Default|GetAttackMagnitude) 1.1)) _projectilespeed)))))

(event Collision|EventActorBeginOverlap
  (params (OtherActor :type Actor%20Object%20Reference)))

(event EventTick
  (params (DeltaSeconds :type Float%20%28single-precision%29))
  (CallFunction|Accelerate DeltaSeconds)
  (Networking|ForceNetUpdate))

(fn ConstructionScript)