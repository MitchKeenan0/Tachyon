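; BP_Volta is a character Blueprint for Volta that keeps a text component and an after-image effect following the character.
; BeginPlay adds a particle system component.
; Each Tick moves TextComponent to a fixed world-space offset from the actor.
; When AfterImages is valid, Tick also places it slightly ahead of the actor along CharacterMovement velocity.
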(event EventBeginPlay
  (AddComponent|AddParticleSystemComponent false))

(event Collision|EventActorBeginOverlap
  (params (OtherActor :type Actor%20Object%20Reference)))

(event EventTick
  (params (DeltaSeconds :type Float%20%28single-precision%29))
  (bind _returnvalue (Transformation|GetActorLocation))
  (bind _afterimages (Variables|Default|GetAfterImages))
  (Transformation|SetWorldLocation (Variables|Default|GetTextComponent) (+ _returnvalue (Math|Vector|MakeVector 0.0 -2.5e+02 -55.0)) false false)
  (Utilities|IsValid _afterimages
    (:Is%20Valid
      (Transformation|SetWorldLocation _afterimages (+ _returnvalue (* (Variables|/Script/Engine.MovementComponent|GetVelocity (Variables|Character|GetCharacterMovement)) 0.02)) false false))))

(fn ConstructionScript)