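; BP_Namacorigean is a character Blueprint with a text component and a test afterimage particle effect.
; After a very brief delay on BeginPlay, it adds a particle system component and sets a white color parameter on TestAfterImages, with no parameter name.
; Each Tick holds the text at a fixed world-space offset from the actor.
; Velocity-based afterimage positioning and a material parameter call are present but never run.
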(event EventBeginPlay
  (Utilities|FlowControl|Delay 0.01)
  (if true
    (AddComponent|AddParticleSystemComponent false)
    (Effects|Components|ParticleSystem|SetColorParameter (Variables|Default|GetTestAfterImages) "None" "(R=1.000000,G=1.000000,B=1.000000,A=1.000000)")))

(event EventTick
  (params (DeltaSeconds :type Float%20%28single-precision%29))
  (Transformation|SetWorldLocation (Variables|Default|GetTextComponent) (+ (Transformation|GetActorLocation) "0,-250.000000,-55.000000") false false))

(fn ConstructionScript)