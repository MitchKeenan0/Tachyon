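; BP_SwarmAttack is a swarm unit that homes in on the GammaCharacter tagged "SwarmCentre".
; BeginPlay randomizes its move speed and interval, so each instance moves differently.
; Tick searches all GammaCharacters until it has a valid target, then runs a timer that periodically steers toward it.
; Each step adds a randomly jittered pull toward the target to the projectile component's velocity, clamped to a maximum speed.
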(event Custom|GetPlayer
  ;[0 0 0] Get Player
  (bind _outactors (Actor|GetAllActorsOfClass "/Script/Gamma.GammaCharacter"))
  (for _array_element _outactors
    (Utilities|IsValid _array_element
      (:Is%20Valid
        (if (Actor|ActorHasTag _array_element "SwarmCentre")
          (Variables|Default|SetPlayer _array_element))))))

(event Custom|MoveToPlayer
  (params (DeltaT :type Float%20%28single-precision%29))
  (bind _player (Variables|Default|GetPlayer))
  (bind _projectilecomponent (Variables|Default|GetProjectileComponent))
  ;[0 0 0] Move To Player
  (bind _output_get (Variables|Default|SetMoveTimer (+ DeltaT (Variables|Default|GetMoveTimer))))
  (if (>= _output_get (Variables|Default|GetMoveTime))
    (Variables|Default|SetMoveTimer 0.0)
    (Utilities|IsValid _projectilecomponent
      (:Is%20Valid
        (Utilities|IsValid _player
          (:Is%20Valid
            (Variables|/Script/Engine.MovementComponent|SetVelocity _projectilecomponent (Math|Vector|ClampVectorSize (+ (* (* (+ (* (Math|Random|RandomUnitVector) 1e+02) (- (Transformation|GetActorLocation _player) (Transformation|GetActorLocation))) (Variables|Default|GetMoveSpeed)) 0.5) (Variables|/Script/Engine.MovementComponent|GetVelocity _projectilecomponent)) 0.0 (Variables|Default|GetProjectileMaxSpeed)))))))))

(event EventBeginPlay
  ;[0 0 0] Init Random MoveSpeed
  (Variables|Default|SetMoveSpeed (+ (* (Variables|Default|GetMoveSpeed) (Math|Random|RandomFloat)) 0.1))
  ;[0 0 0] Init Random MoveTime
  (Variables|Default|SetMoveTime (* (Variables|Default|GetMoveTime) (+ (Math|Random|RandomFloat) 1.0))))

(event Collision|EventActorBeginOverlap
  (params (OtherActor :type Actor%20Object%20Reference)))

(event EventTick
  (params (DeltaSeconds :type Float%20%28single-precision%29))
  (Utilities|IsValid (Variables|Default|GetPlayer)
    (:Is%20Valid
      (CallFunction|MovetoPlayer DeltaSeconds))
    (:Is%20Not%20Valid
      (CallFunction|GetPlayer))))

(fn ConstructionScript)