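; BP_SwordAttack is a server-driven sword swing attack with a blade that extends and retracts as it sweeps.
; Each authority tick scales the sprite's X, growing before half the lifespan and shrinking after, and pitches the attack scene by shot direction.
; Near the end of DynamicLifetime it calls NullifyAttack on the owning BP_GammaCharacter and destroys itself; until then it forces net updates.
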(event Custom|sword%20swing
  (params (DeltaT :type Float%20%28single-precision%29))
  (bind _attacksprite (Variables|Default|GetAttackSprite))
  (bind _attackscene (Variables|Default|GetAttackScene))
  (bind _relativerotation (Variables|/Script/Engine.SceneComponent|GetRelativeRotation _attackscene))
  (bind _relativescale3d (Variables|/Script/Engine.SceneComponent|GetRelativeScale3D _attacksprite))
  (bind (_roll _pitch _yaw) (Math|Rotator|BreakRotator _relativerotation))
  (bind (_x _y _z) (Math|Vector|BreakVector _relativescale3d))
  ;[0 0 0] Determine if we're growing / shrinking the blade this frame
  (if (< (Variables|Default|GetLifeTimer) (/ (Actor|GetLifeSpan) 2.0))
    (Variables|Default|SetSwordGrowDirection 1.0)
    (else
      (Variables|Default|SetSwordGrowDirection -1.0)))
  (Transformation|SetRelativeScale3D (Variables|Default|GetAttackSprite) (Math|Vector|MakeVector (Math|Float|Clamp(Float) (+ (* (Variables|Default|GetSwordGrowDirection) (Variables|Default|GetSwordGrowSpeed) DeltaT) _x) 1.0 (* (Variables|Default|GetSwordLength) 1.0)) _y _z))
  ;[0 0 0] Blade swing
  (Transformation|SetRelativeRotation (Variables|Default|GetAttackScene) (Math|Rotator|MakeRotator _roll (+ (* (Variables|Default|GetShotDirection) (Variables|Default|GetAngleSweep) DeltaT) _pitch) _yaw) false false))

(event EventBeginPlay
  (Networking|SwitchHasAuthority
    (:Authority
      ;[0 0 0] Initialize sword growth speed
      (Variables|Default|SetSwordGrowSpeed (* (Variables|Default|GetSwordGrowSpeed) 1.0))
      (Variables|Default|SetbInitialized true))))

(event EventTick
  (params (DeltaSeconds :type Float%20%28single-precision%29))
  (if (Variables|Default|GetbInitialized)
    (Networking|SwitchHasAuthority
      (:Authority
        (CallFunction|SwordSwing DeltaSeconds)
        ;[0 0 0] Check if lifetime is up
        (if (>= (Variables|Default|GetLifeTimer) (* (Variables|Default|GetDynamicLifetime) 0.98))
          ;[0 0 0] Set pointer null for character, then destroy
          (bind _asbp_gamma_character (Utilities|Casting|CastToBP_GammaCharacter (Variables|Default|GetOwningShooter)))
          (Class|GammaCharacter|NullifyAttack _asbp_gamma_character)
          (Actor|DestroyActor)
          (else
            (Networking|ForceNetUpdate)))))))

(fn ConstructionScript)

(fn OnRepBInitialized)