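; BP_SoccerCube is a physics cube that chases the player while only one GammaCharacter exists and destroys itself when more are present.
; Each tick it recounts GammaCharacters, then applies a constant force toward the first one found.
; A SpinKickInitialize event adds spinning torque, with no caller in this graph.
; Overlaps on SoftCollider activate audio unless the other actor is tagged Attack.
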(event OnComponentBeginOverlap(SoftCollider)
  (params (OverlappedComponent :type Primitive%20Component%20Object%20Reference) (OtherActor :type Actor%20Object%20Reference) (OtherComp :type Primitive%20Component%20Object%20Reference) (OtherBodyIndex :type Integer) (bFromSweep :type Boolean) (SweepResult :type Hit%20Result%20Structure%20%28by%20ref%29))
  (if (not (Actor|ActorHasTag OtherActor "Attack"))
    (Components|Activation|Activate (Variables|Default|GetAudio) false)))

(event Custom|SpinKickInitialize
  (Class|PrimitiveComponent|AddTorqueinDegrees (Variables|Debug|GetStaticMeshComponent) "10000.000000,0.000000,20000.000000" "None" true))

(event Custom|GetPlayersNum
  (bind _outactors (Actor|GetAllActorsOfClass "/Script/Gamma.GammaCharacter"))
  (Variables|Default|SetPlayer1 (Utilities|Array|Get(acopy) _outactors))
  (Variables|Default|SetNumPlayers (Utilities|Array|Length _outactors)))

(event Custom|ApproachPlayer
  (Physics|AddForce (Variables|Debug|GetStaticMeshComponent) (* (Math|Vector|Normalize (- (Transformation|GetActorLocation (Variables|Default|GetPlayer1)) (Transformation|GetActorLocation self))) 2.42e+04) "None" false))

(event EventBeginPlay)

(event Collision|EventActorBeginOverlap
  (params (OtherActor :type Actor%20Object%20Reference)))

(event EventTick
  (params (DeltaSeconds :type Float%20%28single-precision%29))
  (CallFunction|GetPlayersNum)
  (if (> (Variables|Default|GetNumPlayers) 1)
    (Actor|DestroyActor)
    (else
      (Utilities|IsValid (Variables|Default|GetPlayer1)
        (:Is%20Valid
          (CallFunction|ApproachPlayer))))))

(fn ConstructionScript)