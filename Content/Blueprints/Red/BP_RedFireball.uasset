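; BP_RedFireball is Red's fireball actor, which shakes nearby cameras on spawn and expires near the end of its duration.
; BeginPlay plays a light world camera shake at its location with a very large outer radius.
; Each Tick compares LifeTimer to 90% of DurationTime, then calls NullifySecondary on the owning GammaCharacter and destroys itself.
; Destruction only runs if the OwningShooter cast succeeds, and no movement or hit logic is defined here.
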(event EventBeginPlay
  ;[0 0 0] Camera Shake
  (Camera|PlayWorldCameraShake "/Game/Blueprints/GammaFlow/BP_LightCameraShake.BP_LightCameraShake_C" (Transformation|GetActorLocation) 0.0 9999.0))

(event Collision|EventActorBeginOverlap
  (params (OtherActor :type Actor%20Object%20Reference)))

(event EventTick
  (params (DeltaSeconds :type Float%20%28single-precision%29))
  (if (>= (Variables|Default|GetLifeTimer) (* (Variables|Default|GetDurationTime) 0.9))
    (bind _asgamma_character (Utilities|Casting|CastToGammaCharacter (Variables|Default|GetOwningShooter)))
    (Class|GammaCharacter|NullifySecondary _asgamma_character)
    (Actor|DestroyActor)))

(fn ConstructionScript)