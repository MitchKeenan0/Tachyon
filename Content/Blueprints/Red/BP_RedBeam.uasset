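; BP_RedBeam is a sprite-based beam attack actor with a timed lethal window.
; On BeginPlay it spawns a BP_TestBurst muzzle burst at AttackScene, attaches it to itself and plays a strong world camera shake.
; Tick accumulates SpriteTimer, thinning AttackSprite's Z scale toward zero and hiding it once LethalTime is exceeded, unless Finished is set.
; No damage or collision logic appears in these graphs.
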(event EventBeginPlay
  ;[0 0 0] Spawn 'musket' burst
  (bind _returnvalue (Game|SpawnActorfromClass "/Game/Blueprints/Red/BP_TestBurst.BP_TestBurst_C" (Transformation|GetWorldTransform (Variables|Default|GetAttackScene)) "Undefined" 0 0))
  (bind _output_get (Variables|Default|SetBurst _returnvalue))
  (Transformation|AttachActorToActor _output_get self "None" "KeepWorld" "KeepWorld" "KeepRelative" true)
  ;[0 0 0] Camera Shake
  (Camera|PlayWorldCameraShake "/Game/Blueprints/GammaFlow/BP_StrongCameraShake.BP_StrongCameraShake_C" (Transformation|GetActorLocation) 0.0 2e+03))

(event Collision|EventActorBeginOverlap
  (params (OtherActor :type Actor%20Object%20Reference)))

(event EventTick
  (params (DeltaSeconds :type Float%20%28single-precision%29))
  (bind _attacksprite (Variables|Default|GetAttackSprite))
  (bind _relativescale3d (Variables|/Script/Engine.SceneComponent|GetRelativeScale3D _attacksprite))
  (bind (_x _y _z) (Math|Vector|BreakVector _relativescale3d))
  ;[0 0 0] Timing
  (Variables|Default|SetSpriteTimer (+ DeltaSeconds (Variables|Default|GetSpriteTimer)))
  ;[0 0 0] I'mNotDone.mp3
  (if (and (> (Variables|Default|GetSpriteTimer) (Variables|Default|GetLethalTime)) (not (Variables|Default|GetbFinished)))
    ;[0 0 0] Go Invisible, lethal time is over
    (Rendering|SetVisibility (Variables|Default|GetAttackSprite) false false)
    (else
      ;[0 0 0] Thin-out vertical for end of Lethal Time
      (Transformation|SetRelativeScale3D (Variables|Default|GetAttackSprite) (Math|Vector|MakeVector _x _y (Math|Interpolation|FInterptoConstant _z 0.0 DeltaSeconds 1e+01))))))

(fn ConstructionScript)

(fn OnRepInitialRotation)