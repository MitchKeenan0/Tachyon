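; BP_SpearAttack is a spear attack projectile that speeds up as it flies away from its owning shooter.
; At normal time dilation, each Tick compounds its velocity, so acceleration is frame-rate dependent, and calls Nullify beyond a set distance from the shooter.
; Under strong global slow motion it skips acceleration and that range check, enabling forced sub-stepping instead.
; Both branches force a net update every Tick.
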(event Custom|Accelerate
  (bind _projectilecomponent (Variables|Default|GetProjectileComponent))
  (Variables|/Script/Engine.MovementComponent|SetVelocity _projectilecomponent (* (Variables|/Script/Engine.MovementComponent|GetVelocity _projectilecomponent) 1.2))
  (if (>= (Transformation|GetDistanceTo (Variables|Default|GetOwningShooter)) 6e+03)
    (Class|GAttack|Nullify)))

(event EventBeginPlay)

(event Collision|EventActorBeginOverlap
  (params (OtherActor :type Actor%20Object%20Reference)))

(event EventTick
  (params (DeltaSeconds :type Float%20%28single-precision%29))
  (if (> (Class|GameplayStatics|GetGlobalTimeDilation) 0.5)
    (CallFunction|Accelerate)
    (Networking|ForceNetUpdate)
    (else
      (Variables|/Script/Engine.ProjectileMovementComponent|SetbForceSubStepping (Variables|Default|GetProjectileComponent) true)
      (Networking|ForceNetUpdate))))

(fn ConstructionScript)