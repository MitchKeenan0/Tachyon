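; Eye beam actor that spawns a BP_TestBurst at its own transform on BeginPlay and visually jitters while active.
; On Tick, a small timer periodically resets its rotation to the initial one plus a random pitch offset scaled by AttackMagnitude, producing a shake.
; InitialRotation, captured at BeginPlay, has an OnRep handler that is empty, and a debug print is left unconnected.
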(event EventBeginPlay
  (Variables|Default|SetInitialRotation (Transformation|GetActorRotation))
  (bind _returnvalue (Game|SpawnActorfromClass "/Game/Blueprints/BP_TestBurst.BP_TestBurst_C" (Transformation|GetActorTransform) "Undefined" 0 0))
  (Variables|Default|SetBurst _returnvalue))

(event Collision|EventActorBeginOverlap
  (params (OtherActor :type Actor%20Object%20Reference)))

(event EventTick
  (params (DeltaSeconds :type Float%20%28single-precision%29))
  (bind _initialrotation (Variables|Default|GetInitialRotation))
  (bind (_roll _pitch _yaw) (Math|Rotator|BreakRotator _initialrotation))
  (bind _output_get (Variables|Default|SetScaleTimer (+ DeltaSeconds (Variables|Default|GetScaleTimer))))
  (if (>= _output_get 0.02)
    (Variables|Default|SetScaleTimer 0.0)
    (Transformation|SetActorRotation (Math|Rotator|MakeRotator _roll (+ _pitch (* (Math|Random|RandomFloatinRange -1.0 1.0) (Variables|Default|GetAttackMagnitude))) _yaw))))

(fn ConstructionScript)

(fn OnRepInitialRotation)