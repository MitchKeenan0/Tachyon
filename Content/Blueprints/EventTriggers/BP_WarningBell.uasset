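; BP_WarningBell is a flashing text warning that places itself relative to the GammaCharacter when spawned.
; Shortly after BeginPlay, it moves to the first found character's X position at a fixed Y and Z, without following afterward.
; Tick accumulates time and toggles the TextRender's visibility at a short, regular interval to make it blink.
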(event EventBeginPlay
  (Utilities|FlowControl|Delay 0.05)
  (bind _outactors (Actor|GetAllActorsOfClass "/Script/Gamma.GammaCharacter"))
  (if (> (Utilities|Array|Length _outactors) 0)
    (Transformation|SetActorLocation (Math|Vector|MakeVector (.X (Math|Vector|BreakVector (Transformation|GetActorLocation (Utilities|Array|Get(acopy) _outactors)))) 0.0 -1e+02) false false)))

(event Collision|EventActorBeginOverlap
  (params (OtherActor :type Actor%20Object%20Reference)))

(event EventTick
  (params (DeltaSeconds :type Float%20%28single-precision%29))
  (bind _output_get (Variables|Default|SetFlashTimer (+ DeltaSeconds (Variables|Default|GetFlashTimer))))
  (if (>= _output_get 0.1)
    (bind _output_get_2 (Variables|Default|SetbVis (not (Variables|Default|GetbVis))))
    (Rendering|SetVisibility (Variables|Default|GetTextRender) _output_get_2 false)
    (Variables|Default|SetFlashTimer 0.0)))

(fn ConstructionScript)