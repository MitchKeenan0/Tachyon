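; BP_SwordThrow is a thrown sword projectile that flies out and returns to its shooter like a boomerang.
; The server interpolates it at constant speed toward a forward point set at spawn, then after half a second homes on OwningShooter, forcing net updates.
; Overlapping the shooter on return calls NullifySecondary on BP_GammaCharacter and destroys the sword.
; An older velocity-based homing calculation remains unused.
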(event OnComponentBeginOverlap(Box)
  (params (OverlappedComponent :type Primitive%20Component%20Object%20Reference) (OtherActor :type Actor%20Object%20Reference) (OtherComp :type Primitive%20Component%20Object%20Reference) (OtherBodyIndex :type Integer) (bFromSweep :type Boolean) (SweepResult :type Hit%20Result%20Structure%20%28by%20ref%29))
  ;[0 0 0] Destroy on return to shooter
  (if (and (>= (Variables|Default|GetActualLifetime) 0.5) (== OtherActor (Variables|Default|GetOwningShooter)))
    (bind _asbp_gamma_character (Utilities|Casting|CastToBP_GammaCharacter (Variables|Default|GetOwningShooter)))
    (Class|GammaCharacter|NullifySecondary _asbp_gamma_character)
    (Actor|DestroyActor)))

(event EventBeginPlay
  ;[0 0 0] Initial outbound vector
  (Networking|SwitchHasAuthority
    (:Authority
      (Variables|Default|SetFlightVector (+ (Transformation|GetActorLocation) (* (Transformation|GetActorForwardVector) (Variables|Default|GetThrowRange))))
      (Networking|ForceNetUpdate))))

(event EventTick
  (params (DeltaSeconds :type Float%20%28single-precision%29))
  (Networking|SwitchHasAuthority
    (:Authority
      ;[0 0 0] Deliberate when to turn back
      (Variables|Default|SetDeltaT DeltaSeconds)
      (Variables|Default|SetActualLifetime (+ (Variables|Default|GetDeltaT) (Variables|Default|GetActualLifetime)))
      (if (>= (Variables|Default|GetActualLifetime) 0.5)
        ;[0 0 0] Inbound movement
        (Transformation|SetActorLocation (Math|Interpolation|VInterptoConstant (Transformation|GetActorLocation) (Transformation|GetActorLocation (Variables|Default|GetOwningShooter)) (Variables|Default|GetDeltaT) (Variables|Default|GetFlightSpeed)) false false)
        (Networking|ForceNetUpdate)
        (else
          ;[0 0 0] Outbound movement
          (Transformation|SetActorLocation (Math|Interpolation|VInterptoConstant (Transformation|GetActorLocation) (Variables|Default|GetFlightVector) (Variables|Default|GetDeltaT) (Variables|Default|GetFlightSpeed)) false false)
          (Networking|ForceNetUpdate))))))

(fn ConstructionScript)

(fn OnRepBInitialized)