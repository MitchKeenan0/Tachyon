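; BP_Chunk_D is a physics chunk that drifts back toward the player when it gets too far away.
; Each tick it finds the first GammaCharacter and applies acceleration-based force toward it only beyond a distance threshold.
; SoftCollider overlaps with actors not tagged "Attack" activate its audio.
; A size-triggered split into smaller BP_Chunk actors on the Y=0 plane and a random torque are present but never run.
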(event OnComponentBeginOverlap(SoftCollider)
  (params (OverlappedComponent :type Primitive%20Component%20Object%20Reference) (OtherActor :type Actor%20Object%20Reference) (OtherComp :type Primitive%20Component%20Object%20Reference) (OtherBodyIndex :type Integer) (bFromSweep :type Boolean) (SweepResult :type Hit%20Result%20Structure%20%28by%20ref%29))
  (Utilities|IsValid OtherActor
    (:Is%20Valid
      (if (not (Actor|ActorHasTag OtherActor "Attack"))
        (Components|Activation|Activate (Variables|Default|GetAudio) false)))))

(event Custom|GetPlayersNum
  (bind _outactors (Actor|GetAllActorsOfClass "/Script/Gamma.GammaCharacter"))
  (Variables|Default|SetPlayer1 (Utilities|Array|Get(acopy) _outactors))
  (Variables|Default|SetNumPlayers (Utilities|Array|Length _outactors)))

(event Custom|ApproachPlayer
  (bind _self self)
  (bind _player1 (Variables|Default|GetPlayer1))
  (bind _returnvalue (Transformation|GetActorLocation _player1))
  (bind _returnvalue_2 (Transformation|GetActorLocation _self))
  (bind _returnvalue_3 (- _returnvalue _returnvalue_2))
  (Utilities|IsValid (Variables|Debug|GetStaticMeshComponent)
    (:Is%20Valid
      (if (>= (Math|Vector|VectorLength _returnvalue_3) 3e+03)
        (Physics|AddForce (Variables|Debug|GetStaticMeshComponent) (* (Math|Vector|Normalize _returnvalue_3) 1e+02) "None" true)))))

(event Custom|UpdateProgeny
  (bind _returnvalue (Transformation|GetActorLocation))
  (bind _returnvalue_2 (Math|Random|RandomUnitVector))
  (bind _returnvalue_3 (Math|Random|RandomFloatinRange 25.0 5e+01))
  (bind _cubemaxsize (Variables|Default|GetCubeMaxSize))
  (bind _returnvalue_4 (* _returnvalue_2 _returnvalue_3))
  (bind _returnvalue_5 (+ _returnvalue _returnvalue_4))
  (bind (_x _y _z) (Math|Vector|BreakVector _returnvalue_5))
  (if (and (>= (Math|Vector|VectorLength (Transformation|GetActorScale3D)) (Math|Vector|VectorLength (Math|Vector|MakeVector _cubemaxsize _cubemaxsize _cubemaxsize))) (Variables|Default|GetbDoChildOne))
    (for _index (range 0 2)
      (bind _returnvalue_6 (Game|SpawnActorfromClass "/Game/Blueprints/BP_Chunk.BP_Chunk_C" (Math|Transform|MakeTransform (Math|Vector|MakeVector _x 0.0 _z) (Transformation|GetActorRotation) "0.300000,0.300000,0.300000") "Undefined" 0 0))
      (Class|PrimitiveComponent|SetMassScale (Variables|/Script/Engine.StaticMeshActor|GetStaticMeshComponent _returnvalue_6) "None" 1.0)
      (Class|PrimitiveComponent|SetLinearDamping (Variables|/Script/Engine.StaticMeshActor|GetStaticMeshComponent _returnvalue_6) 1.0)
      (Variables|Default|SetbDoChildOne false)
      (Actor|DestroyActor))))

(event EventBeginPlay)

(event Collision|EventActorBeginOverlap
  (params (OtherActor :type Actor%20Object%20Reference)))

(event EventTick
  (params (DeltaSeconds :type Float%20%28single-precision%29))
  ;[0 0 0] Attract to Player
  (CallFunction|GetPlayersNum)
  (if (> (Variables|Default|GetNumPlayers) 0)
    (Utilities|IsValid (Variables|Default|GetPlayer1)
      (:Is%20Valid
        (CallFunction|ApproachPlayer)))))

(fn ConstructionScript)