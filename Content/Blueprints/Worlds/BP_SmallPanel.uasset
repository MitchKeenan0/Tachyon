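; BP_SmallPanel is a world actor that randomizes its own size and placement when play begins.
; BeginPlay gives RenderComponent a random, non-uniform world scale on all three axes.
; It then moves the actor without sweep to a random, widely scaled position across the X-Z plane, with Y effectively fixed.
; The construction script is empty, and overlap and tick events are unused.
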(event EventBeginPlay
  (Transformation|SetWorldScale3D (Variables|Default|GetRenderComponent) (Math|Vector|MakeVector (Math|Random|RandomFloatinRange 1.0 1e+01) (Math|Random|RandomFloatinRange 1.0 1e+01) (Math|Random|RandomFloatinRange 1.0 1e+01)))
  (Transformation|SetActorLocation (* (Math|Vector|MakeVector (Math|Random|RandomFloatinRange -1e+04 1e+04) (Math|Random|RandomFloatinRange 5.0 5.0) (Math|Random|RandomFloatinRange -1e+04 1e+04)) 5e+02) false false))

(event Collision|EventActorBeginOverlap
  (params (OtherActor :type Actor%20Object%20Reference)))

(event EventTick
  (params (DeltaSeconds :type Float%20%28single-precision%29)))

(fn ConstructionScript)