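; Melee sword attack actor that swings a growing blade sprite in an arc, with a camera shake on spawn.
; Once initialized and lethal, it sets blade offset, swing speed and radial force from attack magnitude and shot direction.
; The server then extends the blade, retracts it late in its duration and eases the swing speed down.
; Each server tick matches the capsule collider to the sprite and forces a net update.
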(event Custom|sword%20swing
  (params (DeltaT :type Float%20%28single-precision%29))
  (bind _attacksprite (Variables|Default|GetAttackSprite))
  (bind _attacksprite_2 (Variables|Default|GetAttackSprite))
  (bind _attackscene (Variables|Default|GetAttackScene))
  (bind _relativerotation (Variables|/Script/Engine.SceneComponent|GetRelativeRotation _attackscene))
  (bind _relativescale3d (Variables|/Script/Engine.SceneComponent|GetRelativeScale3D _attacksprite_2))
  (bind (_roll _pitch _yaw) (Math|Rotator|BreakRotator _relativerotation))
  (bind (_x _y _z) (Math|Vector|BreakVector _relativescale3d))
  ;[0 0 0] Determine if we're growing / shrinking the blade this frame
  (if (< (Variables|Default|GetLifeTimer) (* (Variables|Default|GetDurationTime) 0.6))
    (Variables|Default|SetSwordGrowDirection 1.0)
    (else
      (Variables|Default|SetSwordGrowDirection -1.0)))
  (Transformation|SetRelativeScale3D (Variables|Default|GetAttackSprite) (Math|Vector|MakeVector (Math|Float|Clamp(Float) (+ (* (Variables|Default|GetSwordGrowDirection) (Variables|Default|GetSwordGrowSpeed) DeltaT) _x) 2.25 (+ (* (Variables|Default|GetSwordLength) (Variables|Default|GetAttackMagnitude)) (Variables|Default|GetAttackMagnitude))) _y (Math|Float|Clamp(Float) (+ (* (Variables|Default|GetSwordGrowDirection) (Variables|Default|GetSwordGrowSpeed) DeltaT) _z) 1.0 (* 0.3 (* (Variables|Default|GetSwordLength) (+ (Variables|Default|GetAttackMagnitude) 1.0))))))
  ;[0 0 0] Blade swing
  (Transformation|SetRelativeRotation (Variables|Default|GetAttackScene) (Math|Rotator|MakeRotator _roll (+ (* (Variables|Default|GetShotDirection) (Variables|Default|GetSwingSpeed) DeltaT (+ (Math|Float|Clamp(Float) (Variables|Default|GetAttackMagnitude) 0.25 0.5) 0.5)) _pitch) _yaw) true false)
  (Variables|Default|SetSwingSpeed (Math|Interpolation|FInterpTo (Variables|Default|GetSwingSpeed) 15.0 DeltaT 6.18))
  ;[0 0 0] Update capsule collider to match sprite
  (Transformation|SetRelativeLocation (Variables|Default|GetCapsuleRoot) (Variables|/Script/Engine.SceneComponent|GetRelativeLocation _attacksprite) true false)
  (Transformation|SetRelativeRotation (Variables|Default|GetCapsuleRoot) (Variables|/Script/Engine.SceneComponent|GetRelativeRotation _attacksprite) false false)
  (Transformation|SetRelativeScale3D (Variables|Default|GetCapsuleRoot) (Variables|/Script/Engine.SceneComponent|GetRelativeScale3D _attacksprite)))

(event EventBeginPlay
  (Networking|SwitchHasAuthority
    (:Authority
      ;[0 0 0] Initialize sword growth speed
      (Variables|Default|SetSwordGrowSpeed (* (Variables|Default|GetSwordGrowSpeed) 1.0))
      (Variables|Default|SetbInitialized true)
      (Transformation|SetRelativeScale3D (Variables|Default|GetAttackSprite) (Math|Vector|MakeVector 1.0 0.0 1.0))
      ;[0 0 0] Camera Shake
      (Camera|PlayWorldCameraShake "/Game/Blueprints/GammaFlow/BP_LightCameraShake.BP_LightCameraShake_C" (Transformation|GetActorLocation) 0.0 5555.0))))

(event EventTick
  (params (DeltaSeconds :type Float%20%28single-precision%29))
  (bind _radialforce (Variables|Default|GetRadialForce))
  (if (and (Variables|Default|GetbInitialized) (Variables|Default|GetbLethal))
    (if (not (Variables|Default|GetbPositionSet))
      ;[0 0 0] Initialize position
      (Transformation|SetRelativeLocation (Variables|Default|GetAttackSprite) (Math|Vector|MakeVector (+ (* 125.0 (Variables|Default|GetAttackMagnitude)) 75.0) 0.0 (* (Variables|Default|GetShotDirection) 3e+01)) false false)
      (Variables|Default|SetSwingSpeed (Variables|Default|GetAngleSweep))
      (Variables|/Script/Engine.RadialForceComponent|SetForceStrength _radialforce (* (Variables|/Script/Engine.RadialForceComponent|GetForceStrength _radialforce) (+ (Variables|Default|GetAttackMagnitude) 1.0)))
      (Variables|Default|SetbPositionSet true)
      (else
        (Networking|SwitchHasAuthority
          (:Authority
            (CallFunction|SwordSwing DeltaSeconds)
            (Networking|ForceNetUpdate)))))))

(fn ConstructionScript)

(fn OnRepBInitialized)