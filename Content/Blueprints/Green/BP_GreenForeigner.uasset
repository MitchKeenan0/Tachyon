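; BP_GreenForeigner is a character Blueprint for a green "foreigner" with a particle effect and a text component that follows it.
; BeginPlay adds a particle system component to the character.
; Each Tick moves the text component to a fixed world-space offset from the actor's location, independent of facing.
; An unconnected node would place an AfterImage component ahead along the movement velocity, but it never runs.
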(event EventBeginPlay
  (AddComponent|AddParticleSystemComponent false))

(event Collision|EventActorBeginOverlap
  (params (OtherActor :type Actor%20Object%20Reference)))

(event EventTick
  (params (DeltaSeconds :type Float%20%28single-precision%29))
  (Transformation|SetWorldLocation (Variables|Default|GetTextComponent) (+ (Transformation|GetActorLocation) "0,-250.000000,-55.000000") false false))

(fn ConstructionScript)