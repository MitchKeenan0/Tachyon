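; Thrown sword projectile that flies out from its shooter and returns like a boomerang, with a camera shake on spawn.
; The server sets an outbound target on the Y=0 plane, with range and speed influenced by the shooter's velocity.
; After a time or distance limit, it homes on the shooter, accelerating each tick and forcing net updates.
; Overlapping the shooter after a brief delay calls NullifySecondary on the GammaCharacter and destroys the sword.
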(event OnComponentBeginOverlap(ReturnDetecBox)
  (params (OverlappedComponent :type Primitive%20Component%20Object%20Reference) (OtherActor :type Actor%20Object%20Reference) (OtherComp :type Primitive%20Component%20Object%20Reference) (OtherBodyIndex :type Integer) (bFromSweep :type Boolean) (SweepResult :type Hit%20Result%20Structure%20%28by%20ref%29))
  (bind _self self)
  ;[0 0 0] Destroy on return to shooter
  (if (and (>= (Variables|Default|GetActualLifetime) 0.2) (== OtherActor (Variables|Default|GetOwningShooter)))
    (bind _asgamma_character (Utilities|Casting|CastToGammaCharacter (Variables|Default|GetOwningShooter)))
    (Class|GammaCharacter|NullifySecondary _asgamma_character)
    (Utilities|IsValid _self
      (:Is%20Valid
        (Actor|DestroyActor _self)))))

(event EventBeginPlay
  ;[0 0 0] Camera Shake
  (Camera|PlayWorldCameraShake "/Game/Blueprints/GammaFlow/BP_LightCameraShake.BP_LightCameraShake_C" (Transformation|GetActorLocation) 0.0 6666.0))

(event EventTick
  (params (DeltaSeconds :type Float%20%28single-precision%29))
  (bind _returnvalue (Transformation|GetActorLocation))
  (bind _returnvalue_2 (Transformation|GetActorForwardVector))
  (bind _owningshooter (Variables|Default|GetOwningShooter))
  (bind _throwrange (Variables|Default|GetThrowRange))
  (bind _returnvalue_3 (Transformation|GetVelocity _owningshooter))
  (bind _returnvalue_4 (Math|Vector|VectorLength _returnvalue_3))
  (bind _returnvalue_5 (* _returnvalue_4 1.0))
  (bind _returnvalue_6 (* _throwrange _returnvalue_5))
  (bind _returnvalue_7 (* _returnvalue_2 _returnvalue_6))
  (bind _returnvalue_8 (+ _returnvalue _returnvalue_7))
  (bind (_x _y _z) (Math|Vector|BreakVector _returnvalue_8))
  (Networking|SwitchHasAuthority
    (:Authority
      (Utilities|IsValid (Variables|Default|GetOwningShooter)
        (:Is%20Valid
          (if (not (Variables|Default|GetbInitialized))
            ;[0 0 0] Initial outbound vector
            (Variables|Default|SetFlightVector (Math|Vector|MakeVector _x 0.0 _z))
            (Components|Activation|Activate (Variables|Default|GetRotatingMovement) false)
            (Variables|Default|SetbInitialized true)
            (Networking|ForceNetUpdate)
            (else
              ;[0 0 0] Deliberate when to turn back
              (Variables|Default|SetDeltaT DeltaSeconds)
              (Variables|Default|SetActualLifetime (+ (Variables|Default|GetDeltaT) (Variables|Default|GetActualLifetime)))
              (if (or (>= (Variables|Default|GetActualLifetime) 0.5) (>= (Transformation|GetDistanceTo (Variables|Default|GetOwningShooter)) (Variables|Default|GetMaxDistance)))
                ;[0 0 0] Inbound movement
                (Transformation|SetActorLocation (Math|Interpolation|VInterptoConstant (Transformation|GetActorLocation) (Transformation|GetActorLocation (Variables|Default|GetOwningShooter)) (Variables|Default|GetDeltaT) (Variables|Default|GetFlightSpeed)) true false)
                ;;[0 0 0] Accelerating Return Speed
                (Variables|Default|SetFlightSpeed (* (Variables|Default|GetFlightSpeed) 1.01))
                (Networking|ForceNetUpdate)
                (else
                  ;[0 0 0] Outbound movement
                  (Transformation|SetActorLocation (Math|Interpolation|VInterptoConstant (Transformation|GetActorLocation) (Variables|Default|GetFlightVector) (Variables|Default|GetDeltaT) (+ (Variables|Default|GetFlightSpeed) (* (Math|Vector|VectorLength (Transformation|GetVelocity (Variables|Default|GetOwningShooter))) 1.0))) true false)
                  (Networking|ForceNetUpdate))))))))))

(fn ConstructionScript)

(fn OnRepBInitialized)