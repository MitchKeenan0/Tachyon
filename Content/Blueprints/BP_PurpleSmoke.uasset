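; Purple smoke puff effect that fires a strong world camera shake on spawn and randomizes its damage sound's pitch.
; BeginPlay gives the Paper2D sprite a random pitch rotation and world Y depth, sets a small starting scale, then detaches it.
; Each Tick interpolates the sprite's scale toward a target re-randomized every frame, giving jittery growth.
; Once the scale's length reaches the target's, it shrinks to zero; the actor is never destroyed here.
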(event Custom|UpdateSprite
  (params (DeltaT :type Float%20%28single-precision%29))
  (bind _papersprite (Variables|Default|GetPaperSprite))
  (bind _targetsize (Variables|Default|GetTargetSize))
  (bind _targetspeed (Variables|Default|GetTargetSpeed))
  (bind _relativescale3d (Variables|/Script/Engine.SceneComponent|GetRelativeScale3D _papersprite))
  (bind _returnvalue (Math|Interpolation|VInterpTo _relativescale3d _targetsize DeltaT _targetspeed))
  ;[0 0 0] UPDATE SPRITE
  (CallFunction|SpriteVectorTiming)
  (Transformation|SetRelativeScale3D _papersprite _returnvalue)
  (if (>= (Math|Vector|VectorLength _returnvalue) (Math|Vector|VectorLength (Variables|Default|GetTargetSize)))
    (Variables|Default|SetbYoungSprite false)))

(event Custom|SpriteVectorTiming
  (bind _returnvalue (Math|Random|RandomFloatinRange 1.0 3.0))
  ;[0 0 0] UPDATE SPRITE
  (if (Variables|Default|GetbYoungSprite)
    (Variables|Default|SetTargetSize (Math|Vector|MakeVector _returnvalue 1.0 _returnvalue))
    (Variables|Default|SetTargetSpeed 5e+01)
    (else
      (Variables|Default|SetTargetSize "0, 0, 0")
      (Variables|Default|SetTargetSpeed 35.0))))

(event EventBeginPlay
  (bind _papersprite (Variables|Default|GetPaperSprite))
  (bind _returnvalue (Transformation|GetWorldLocation _papersprite))
  (bind (_x _y _z) (Math|Vector|BreakVector _returnvalue))
  ;[0 0 0] Init Random TargetSize
  (Variables|Default|SetTargetSize (* (Variables|Default|GetTargetSize) (Math|Random|RandomFloatinRange 0.5 1e+01)))
  ;[0 0 0] Camera Shake
  (Camera|PlayWorldCameraShake "/Game/Blueprints/GammaFlow/BP_StrongCameraShake.BP_StrongCameraShake_C" (Transformation|GetActorLocation) 0.0 2e+03)
  ;[0 0 0] Range-Random Pitch
  (Audio|Components|Audio|SetPitchMultiplier (Variables|Default|GetDamageSound) (Math|Random|RandomFloatinRange 0.15 1.0))
  ;[0 0 0] Initialize Sprite
  (Utilities|IsValid _papersprite
    (:Is%20Valid
      (Transformation|SetRelativeRotation _papersprite (Math|Rotator|MakeRotator 0.0 (Math|Random|RandomFloatinRange 0.0 1.8e+02) 0.0) false false)
      (Transformation|SetWorldLocation _papersprite (Math|Vector|MakeVector _x (Math|Random|RandomFloatinRange -1e+01 -1e+02) _z) false false)
      (Transformation|SetRelativeScale3D _papersprite "0.200000,0.200000,0.200000")
      (Transformation|DetachFromComponent _papersprite "KeepWorld" "KeepRelative" "KeepRelative" true))))

(event Collision|EventActorBeginOverlap
  (params (OtherActor :type Actor%20Object%20Reference)))

(event EventTick
  (params (DeltaSeconds :type Float%20%28single-precision%29))
  ;[0 0 0] TICK
  (Utilities|IsValid (Variables|Default|GetPaperSprite)
    (:Is%20Valid
      (CallFunction|UpdateSprite DeltaSeconds))))

(fn ConstructionScript)